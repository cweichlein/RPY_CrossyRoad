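; Player pawn that hops a fixed distance per WASD press, with chicken-named helpers suggesting a Crossy Road-style character.
; Tick runs Update while alive: ChickController sets direction and jump velocity, then Move, TurnChicken and Jump apply frame-stepped offsets and 90/180-degree yaw turns.
; MoveForward/MoveRight axes also add movement input, and number keys toggle ShipMesh scales or spawn emitters.
; OnDeath hides Collision and its children, then reopens TutorialMap after a delay.
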(event `Key|Four`
  (params (Key :type "Key Structure"))
  (:`Pressed`
    (`/Engine/EditorBlueprintResources/StandardMacros.FlipFlop`
      (:`A`
        (`GameplayStatics.SpawnEmitterAtLocation` null (`self.K2_GetActorLocation`))))))

(event `Key|Three`
  (params (Key :type "Key Structure"))
  (:`Pressed`
    (`/Engine/EditorBlueprintResources/StandardMacros.FlipFlop`
      (:`A`
        (`GameplayStatics.SpawnEmitterAtLocation` null (`self.K2_GetActorLocation`))))))

(event `Key|Two`
  (params (Key :type "Key Structure"))
  (:`Pressed`
    (`/Engine/EditorBlueprintResources/StandardMacros.FlipFlop`
      (:`A`
        (`SceneComponent.SetWorldScale3D` (`self.ShipMesh`) (100.0 125.0 10.0)))
      (:`B`
        (`SceneComponent.SetWorldScale3D` (`self.ShipMesh`) (100.0 100.0 100.0))))))

(event `Key|One`
  (params (Key :type "Key Structure"))
  (:`Pressed`
    (`/Engine/EditorBlueprintResources/StandardMacros.FlipFlop`
      (:`A`
        (`SceneComponent.SetWorldScale3D` (`self.ShipMesh`) (200.0 10.0 100.0)))
      (:`B`
        (`SceneComponent.SetWorldScale3D` (`self.ShipMesh`) (100.0 100.0 100.0))))))

(event `self.ReceiveBeginPlay`
  (set `PlayerController.bShowMouseCursor` true (`GameplayStatics.GetPlayerController` 0))
  (`PrimitiveComponent.SetEnableGravity` (`self.Collision`) true))

(event `self.ReceiveTick`
  (params (DeltaSeconds :type "Float (single-precision)"))
  (`self.Update`))

(event `InputAxis|MoveForward`
  (params (AxisValue :type "Float (single-precision)"))
  (`self.AddMovementInput` (1.0 0.0 0.0) AxisValue))

(event `InputAxis|MoveRight`
  (params (AxisValue :type "Float (single-precision)"))
  (`self.AddMovementInput` (0.0 1.0 0.0) AxisValue))

(event `OnDeath`
  (`|ExecutionSequence`
    (:`then_0`
      (set `self.Dead` true)
      (`SceneComponent.SetVisibility` (`self.Collision`) false true)
      (`KismetSystemLibrary.Delay` 1.0)
      (`GameplayStatics.OpenLevel` "TutorialMap"))))

(fn `ChickController`
  ;[1 1 1] If player can move check movement
  (if (and (`self.canTurn`) (`self.Can_move`))
    ;[1 1 1] Set Prev Direction
    (set `self.Prev_Dir` (`self.Curr_Dir`))
    (if (`PlayerController.WasInputKeyJustPressed` (`GameplayStatics.GetPlayerController` 0) "W")
      (set `self.Curr_Dir` 0)
      (set `self.Can_move` false)
      (set `self.moveVector` (1.0 0.0 0.0))
      (`self.setTurn` :!label _label)
      (set `self.Can_crouch` false)
      (set `self.can_Jump` false)
      (set `self.jumpVelocity` 200.0)
      (elif (`PlayerController.WasInputKeyJustPressed` (`GameplayStatics.GetPlayerController` 0) "S")
        (set `self.Curr_Dir` 1)
        (set `self.Can_move` false)
        (set `self.moveVector` (-1.0 0.0 0.0))
        (goto _label)
        (elif (`PlayerController.WasInputKeyJustPressed` (`GameplayStatics.GetPlayerController` 0) "A")
          (set `self.Curr_Dir` 2)
          (set `self.Can_move` false)
          (set `self.moveVector` (0.0 -1.0 0.0))
          (goto _label)
          (elif (`PlayerController.WasInputKeyJustPressed` (`GameplayStatics.GetPlayerController` 0) "D")
            (set `self.Curr_Dir` 3)
            (set `self.Can_move` false)
            (set `self.moveVector` (0.0 1.0 0.0))
            (goto _label)))))))

(fn `Jump`
  (bind _returnvalue (`GameplayStatics.GetWorldDeltaSeconds`))
  (bind _maxfallspeed (`self.MaxFallSpeed`))
  (bind _returnvalue_2 (`KismetStringLibrary.Conv_DoubleToString` (`self.jumpVelocity`)))
  (bind _returnvalue_3 (- (`self.jumpVelocity`) (* (`self.jumpAcceleration`) (`GameplayStatics.GetWorldDeltaSeconds`))))
  (if (<= _returnvalue_3 _maxfallspeed)
    (bind _output_get (set `self.jumpVelocity` _maxfallspeed))
    (`self.K2_AddActorWorldOffset` (`KismetMathLibrary.MakeVector` 0.0 0.0 (* _output_get _returnvalue)) true)
    (`KismetSystemLibrary.PrintString` _returnvalue_2)
    (else
      (bind _output_get_2 (set `self.jumpVelocity` _returnvalue_3))
      (`self.K2_AddActorWorldOffset` (`KismetMathLibrary.MakeVector` 0.0 0.0 (* _output_get_2 _returnvalue)) true)
      (`KismetSystemLibrary.PrintString` _returnvalue_2))))

(fn `Move`
  (set `self.change in distance` (* (`GameplayStatics.GetWorldDeltaSeconds`) (`self.Speed`)))
  (set `self.total distance` (+ (`self.total distance`) (`self.change in distance`)))
  (if (>= (`self.total distance`) (`self.distance`))
    (`self.K2_AddActorWorldOffset` (* (`self.moveVector`) (- (`self.distance`) (- (`self.total distance`) (`self.change in distance`)))) true)
    (set `self.total distance` 0.0)
    (set `self.Can_move` true)
    (else
      (`self.K2_AddActorWorldOffset` (* (`self.moveVector`) (`self.change in distance`)) true))))

(fn `setTurn`
  ;[1 1 1] if curr == prev do not turn
  (if (== (`self.Prev_Dir`) (`self.Curr_Dir`))
    _
    (elif (== (`self.Prev_Dir`) (`self.Left`))
      (if (== (`self.Curr_Dir`) (`self.Right`))
        (set `self.turnType` 1.0)
        (set `self.turnDirection` -1.0 :!label _label)
        (set `self.canTurn` false :!label _label_2)
        (elif (== (`self.Curr_Dir`) (`self.Down`))
          (set `self.turnType` 0.0)
          (goto _label)
          (elif (== (`self.Curr_Dir`) (`self.Up`))
            (set `self.turnType` 0.0)
            (set `self.turnDirection` 1.0 :!label _label_3)
            (goto _label_2))))
      (elif (== (`self.Prev_Dir`) (`self.Right`))
        (if (== (`self.Curr_Dir`) (`self.Left`))
          (set `self.turnType` 1.0)
          (goto _label_3)
          (elif (== (`self.Curr_Dir`) (`self.Down`))
            (set `self.turnType` 0.0)
            (goto _label_3)
            (elif (== (`self.Curr_Dir`) (`self.Up`))
              (set `self.turnType` 0.0)
              (goto _label))))
        (elif (== (`self.Prev_Dir`) (`self.Down`))
          (if (== (`self.Curr_Dir`) (`self.Right`))
            (set `self.turnType` 0.0)
            (goto _label)
            (elif (== (`self.Curr_Dir`) (`self.Left`))
              (set `self.turnType` 0.0)
              (goto _label_3)
              (elif (== (`self.Curr_Dir`) (`self.Up`))
                (set `self.turnType` 1.0)
                (goto _label_3))))
          (elif (== (`self.Prev_Dir`) (`self.Up`))
            (if (== (`self.Curr_Dir`) (`self.Right`))
              (set `self.turnType` 0.0)
              (goto _label_3)
              (elif (== (`self.Curr_Dir`) (`self.Down`))
                (set `self.turnType` 1.0)
                (goto _label_3)
                (elif (== (`self.Curr_Dir`) (`self.Left`))
                  (set `self.turnType` 0.0)
                  (goto _label))))))))))

(fn `TurnChicken`
  (bind _defaultsceneroot (`self.DefaultSceneRoot`))
  (bind _returnvalue (select `int` (`KismetMathLibrary.FTrunc64` (`self.turnType`)) :`0` (`self.Turn 90`) :`1` (`self.Turn 180`)))
  (set `self.change in turn` (* (`GameplayStatics.GetWorldDeltaSeconds`) _returnvalue 8.0))
  (set `self.turnTotal` (+ (`self.turnTotal`) (`self.change in turn`)))
  (if (>= (`self.turnTotal`) _returnvalue)
    (`SceneComponent.K2_AddWorldRotation` _defaultsceneroot (`KismetMathLibrary.MakeRotator` 0.0 0.0 (* (`self.turnDirection`) (`self.change in turn`))) false false)
    (set `self.turnTotal` 0.0)
    (set `self.canTurn` true)
    (else
      (`SceneComponent.K2_AddWorldRotation` _defaultsceneroot (`KismetMathLibrary.MakeRotator` 0.0 0.0 (* (`self.turnDirection`) (`self.change in turn`))) false false))))

(fn `Update`
  ;[1 1 1] Check if alive
  (if (not (`self.Dead`))
    (`self.ChickController`) ; set move
    (if (not (`self.canTurn`))
      (`self.TurnChicken`))
    ;[1 1 1] Check if can move
    (if (not (`self.Can_move`))
      ;[1 1 1] Move and turn towards direction
      (`self.Move`))
    (if (not (`self.can_Jump`))
      (`self.Jump`))))

(fn `UserConstructionScript`)