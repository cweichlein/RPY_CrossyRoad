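; One lane strip in an endless Crossy Road-style level: grass, road with vehicles, or water with logs and lilypads.
; BeginPlay spawns the ground, positions a trigger box and, except on grass, loops delayed spawns of one random mesh type, mirrored by direction.
; Tick moves these movers along Y and culls the oldest past a limit.
; Player overlap re-enables jumping and, on forward moves, has StripSpawner add a strip and destroys the oldest.
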(event `self.ReceiveBeginPlay`
  (bind _groundtype (`self.GroundType`))
  (bind _roadspawndirection (`self.RoadSpawnDirection`))
  (`self.GetRandGround` _groundtype)
  (bind _outputroadloc (`self.SpawnRoad` _roadspawndirection (`self.InitialRoadPos`)))
  (bind _output_get (set `self.NextStripLocation` (+ _outputroadloc (`KismetMathLibrary.MakeVector` (`self.NextStripDistance`)))))
  (`SceneComponent.K2_SetWorldTransform` (`self.Box`) (`KismetMathLibrary.MakeTransform` (`KismetMathLibrary.MakeVector` (.x _output_get) (- (.y _output_get) 200.0) (+ 100.0 (.z _output_get)))) false true)
  (`self.GetRandVehicle` _groundtype)
  (if (not (== _groundtype 0))
    (bind _vehiclespawnpoint (`self.CreateVehicleSpawn` _outputroadloc _roadspawndirection))
    (`self.SpawnVehicle` _vehiclespawnpoint _roadspawndirection :!label _label)
    (`KismetSystemLibrary.Delay` (`self.SpawnDelay`))
    (goto _label)))

(event `self.ReceiveTick`
  (params (DeltaSeconds :type "Float (single-precision)"))
  (bind _roadspawndirection (`self.RoadSpawnDirection`))
  (if (not (== (`self.GroundType`) 0))
    (`self.MoveVehicles` DeltaSeconds _roadspawndirection)
    (`self.RemoveEarliestVehicle` _roadspawndirection)))

(event `self.Box.OnComponentBeginOverlap`
  (params (OverlappedComponent :type "PrimitiveComponent Object Reference") (OtherActor :type "Actor Object Reference") (OtherComp :type "PrimitiveComponent Object Reference") (OtherBodyIndex :type Integer) (bFromSweep :type Boolean) (SweepResult :type "HitResult Structure (by ref)"))
  (bind _stripspawner (`self.StripSpawner`))
  (bind _strips (`/Game/InfiniteMatrix/Blueprints/StripSpawner.Strips` _stripspawner))
  (bind _output (`|GetArrayItem` _strips))
  (`KismetSystemLibrary.PrintString` (`KismetSystemLibrary.GetDisplayName` OverlappedComponent))
  (bind _asbp_player_1 (cast `/Game/InfiniteMatrix/Blueprints/BP_Player1` OtherActor))
  (if (or (== (`/Game/InfiniteMatrix/Blueprints/BP_Player1.Curr_Dir` _asbp_player_1) (`/Game/InfiniteMatrix/Blueprints/BP_Player1.Right` _asbp_player_1)) (== (`/Game/InfiniteMatrix/Blueprints/BP_Player1.Curr_Dir` _asbp_player_1) (`/Game/InfiniteMatrix/Blueprints/BP_Player1.Left` _asbp_player_1)) (== (`/Game/InfiniteMatrix/Blueprints/BP_Player1.Curr_Dir` _asbp_player_1) (`/Game/InfiniteMatrix/Blueprints/BP_Player1.Down` _asbp_player_1)))
    (set `/Game/InfiniteMatrix/Blueprints/BP_Player1.can_Jump` true _asbp_player_1)
    (else
      (`/Game/InfiniteMatrix/Blueprints/StripSpawner.SpawnStipAtPoint` _stripspawner)
      (set `/Game/InfiniteMatrix/Blueprints/BP_Player1.can_Jump` true _asbp_player_1)
      (`self.DestroyStrip` _output)
      (`KismetArrayLibrary.Array_RemoveItem` _strips _output))))

(fn `CreateVehicleSpawn`
  (params (Location :type "Vector Structure") (Direction :type Boolean))
  (returns (VehicleSpawnPoint :type "Vector Structure"))
  (if Direction
    (bind _output_get (set `self.TruckOffset` -500.0))
    (bind _returnvalue (`|SpawnActorFromClass` "/DatasmithContent/Blueprints/FBXImporter/BP_SceneNode.BP_SceneNode_C" (`KismetMathLibrary.MakeTransform` (`KismetMathLibrary.MakeVector` Location_X (+ Location_Y _output_get) 1.0)) "Undefined" "OverrideRootScale" null null))
    (bind _output_get_2 (set `self.SpawnPoint` _returnvalue))
    (return (`SceneComponent.K2_GetComponentLocation` (`Actor.RootComponent` _output_get_2)))
    (else
      (bind _output_get_3 (set `self.TruckOffset` 200.0))
      (bind _returnvalue_2 (`|SpawnActorFromClass` "/DatasmithContent/Blueprints/FBXImporter/BP_SceneNode.BP_SceneNode_C" (`KismetMathLibrary.MakeTransform` (`KismetMathLibrary.MakeVector` Location_X (+ Location_Y _output_get_3) 1.0)) "Undefined" "OverrideRootScale" null null))
      (bind _output_get_4 (set `self.SpawnPoint` _returnvalue_2))
      (return (`SceneComponent.K2_GetComponentLocation` (`Actor.RootComponent` _output_get_4))))))

(fn `DestroyAllVehicles`
  (bind _vehicles (`self.Vehicles`))
  (for (_array_element _array_index) _vehicles
    (`self.K2_DestroyActor` _array_element)
    (`KismetArrayLibrary.Array_Remove` _vehicles _array_index)))

(fn `DestroyStrip`
  (params (StripToDestroy :type "/Game/InfiniteMatrix/Blueprints/BP_TunnelSpawner Object Reference"))
  (`|ExecutionSequence`
    (:`then_0`
      (set `self.StipDestroyed` true))
    (:`then_1`
      (`self.K2_DestroyActor` (`/Game/InfiniteMatrix/Blueprints/BP_TunnelSpawner.Ground` StripToDestroy)))
    (:`then_2`
      (`self.DestroyAllVehicles` StripToDestroy))
    (:`then_3`
      (`self.K2_DestroyActor` StripToDestroy))))

(fn `GetRandGround`
  (params (MeshType :type Integer))
  (set `self.SelectedGround` (select `int` MeshType :`0` "/Game/InfiniteMatrix/Meshes/grass.grass" :`1` "/Game/InfiniteMatrix/Meshes/full_road.full_road" :`2` "/Game/InfiniteMatrix/Meshes/water.water" :!type "StaticMesh Object Reference")))

(fn `GetRandVehicle`
  (params (GroundType :type Integer))
  (switch `int` GroundType ; 0 : Grass\n1: Road\n2: Water
    (:`1`
      (set `self.SelectedVehicle` (select `int` (`KismetMathLibrary.RandomIntegerInRange` 0 2) :`0` "/Game/InfiniteMatrix/Meshes/blue_truck.blue_truck" :`1` "/Game/InfiniteMatrix/Blueprints/car_blue.car_blue" :`2` "/Game/InfiniteMatrix/Meshes/pickup_truck.pickup_truck" :!type "StaticMesh Object Reference")))
    (:`2`
      (set `self.SelectedVehicle` (select `int` (`KismetMathLibrary.RandomIntegerInRange` 0 1) :`0` "/Game/InfiniteMatrix/Meshes/log_small.log_small" :`1` "/Game/InfiniteMatrix/Meshes/lilypad.lilypad" :!type "StaticMesh Object Reference")))))

(fn `MoveVehicles`
  (params (DeltaSeconds :type "Float (double-precision)") (Direction :type Boolean))
  (for _array_element (`self.Vehicles`)
    (if Direction
      (bind _output_get (set `self.Movespeed` 100.0))
      (`self.K2_AddActorWorldOffset` _array_element (`KismetMathLibrary.MakeVector` 0.0 (* DeltaSeconds _output_get)) true false)
      (else
        (bind _output_get_2 (set `self.Movespeed` -100.0))
        (`self.K2_AddActorWorldOffset` _array_element (`KismetMathLibrary.MakeVector` 0.0 (* DeltaSeconds _output_get_2)) true false)))))

(fn `RemoveEarliestVehicle`
  (params (Direction :type Boolean))
  (bind _vehicles (`self.Vehicles`))
  (bind _output (`|GetArrayItem` _vehicles))
  (bind (_returnvalue_x _returnvalue_y) (`KismetMathLibrary.BreakVector` (`SceneComponent.K2_GetComponentLocation` (`Actor.RootComponent` _output))))
  (if Direction
    (bind _output_get (set `self.DestroyDistance` 500.0))
    (if (>= _returnvalue_y _output_get)
      (`self.K2_DestroyActor` _output :!label _label)
      (`KismetArrayLibrary.Array_RemoveItem` _vehicles _output))
    (else
      (bind _output_get_2 (set `self.DestroyDistance` -800.0))
      (if (<= _returnvalue_y _output_get_2)
        (goto _label)))))

(fn `SpawnRoad`
  (params (SpawnDirection :type Boolean) (InitialRoadPos :type "Vector Structure"))
  (returns (OutputRoadLoc :type "Vector Structure"))
  (locals (ScaleMultiplier :type "Float (double-precision)"))
  (if SpawnDirection
    (bind _returnvalue (`|SpawnActorFromClass` "/Game/InfiniteMatrix/Blueprints/BP_Ground.BP_Ground_C" (`KismetMathLibrary.MakeTransform` InitialRoadPos (struct) (1.0 1.0 1.0)) "Undefined" "OverrideRootScale" null null))
    (bind _output_get (set `self.Ground` _returnvalue))
    (`StaticMeshComponent.SetStaticMesh` (`/Game/InfiniteMatrix/Blueprints/BP_Ground.StaticMesh` _output_get) (`self.SelectedGround`))
    (return (`SceneComponent.K2_GetComponentLocation` (`Actor.RootComponent` _output_get)))
    (else
      (bind _returnvalue_2 (`|SpawnActorFromClass` "/Game/InfiniteMatrix/Blueprints/BP_Ground.BP_Ground_C" (`KismetMathLibrary.MakeTransform` (+ InitialRoadPos (0.0 -500.0 0.0)) (struct) (1.0 -1.0 1.0)) "Undefined" "OverrideRootScale" null null))
      (bind _output_get_2 (set `self.Ground` _returnvalue_2))
      (`StaticMeshComponent.SetStaticMesh` (`/Game/InfiniteMatrix/Blueprints/BP_Ground.StaticMesh` _output_get_2) (`self.SelectedGround`))
      (return (+ (`SceneComponent.K2_GetComponentLocation` (`Actor.RootComponent` _output_get_2)) (0.0 500.0 0.0))))))

(fn `SpawnVehicle`
  (params (SpawnLocation :type "Vector Structure") (Direction :type Boolean))
  (if (`self.StipDestroyed`)
    _
    (elif Direction
      (bind _returnvalue (`|SpawnActorFromClass` "/Game/InfiniteMatrix/Blueprints/BP_Vehicle.BP_Vehicle_C" (`KismetMathLibrary.MakeTransform` (`KismetMathLibrary.MakeVector` SpawnLocation_X SpawnLocation_Y SpawnLocation_Z)) "Undefined" "OverrideRootScale" null null))
      (`StaticMeshComponent.SetStaticMesh` (`/Game/InfiniteMatrix/Blueprints/BP_Vehicle.StaticMesh` _returnvalue) (`self.SelectedVehicle`))
      (`KismetArrayLibrary.Array_Add` (`self.Vehicles`) _returnvalue)
      (else
        (bind _returnvalue_2 (`|SpawnActorFromClass` "/Game/InfiniteMatrix/Blueprints/BP_Vehicle.BP_Vehicle_C" (`KismetMathLibrary.MakeTransform` (`KismetMathLibrary.MakeVector` SpawnLocation_X SpawnLocation_Y SpawnLocation_Z) (struct) (1.0 -1.0 1.0)) "Undefined" "OverrideRootScale" null null))
        (`StaticMeshComponent.SetStaticMesh` (`/Game/InfiniteMatrix/Blueprints/BP_Vehicle.StaticMesh` _returnvalue_2) (`self.SelectedVehicle`))
        (`KismetArrayLibrary.Array_Add` (`self.Vehicles`) _returnvalue_2)))))

(fn `UserConstructionScript`)