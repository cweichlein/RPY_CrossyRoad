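; Player ship pawn that moves on world X/Y and, on death, hides its collision component and reopens TutorialMap after a delay.
; Each Tick while alive, a WASD press sets a direction, snaps rotation on a direction change and applies one swept, Speed-scaled step.
; MoveForward and MoveRight axes also add movement input and toggle the thruster particles.
; The mouse-aim Turn function is left disconnected.
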(event `self.ReceiveBeginPlay`
  (set `PlayerController.bShowMouseCursor` true (`GameplayStatics.GetPlayerController` 0)))

(event `self.ReceiveTick`
  (params (DeltaSeconds :type "Float (single-precision)"))
  (`self.Update`)
  (if (and (== (`self.GetInputAxisValue`) 0.0) (== (`self.GetInputAxisValue`) 0.0))
    (`ActorComponent.Deactivate` (`self.ThrusterParticles`))
    (else
      (`ActorComponent.Activate` (`self.ThrusterParticles`) false))))

(event `InputAxis|MoveForward`
  (params (AxisValue :type "Float (single-precision)"))
  (`self.AddMovementInput` (1.0 0.0 0.0) AxisValue))

(event `InputAxis|MoveRight`
  (params (AxisValue :type "Float (single-precision)"))
  (`self.AddMovementInput` (0.0 1.0 0.0) AxisValue))

(event `OnDeath`
  (`|ExecutionSequence`
    (:`then_0`
      (set `self.Dead` true)
      (`SceneComponent.SetVisibility` (`self.Collision`) false true)
      (`KismetSystemLibrary.Delay` 1.0)
      (`GameplayStatics.OpenLevel` "TutorialMap"))))

(fn `ChickController`
  ;[1 1 1] Set Prev Direction
  (set `self.Prev_Dir` (`self.Curr_Dir`))
  ;[1 1 1] If player can move check movement
  (if (`self.Can_move`)
    (if (`PlayerController.WasInputKeyJustPressed` (`GameplayStatics.GetPlayerController` 0) "W")
      (set `self.Curr_Dir` 0)
      (set `self.Can_move` false)
      (elif (`PlayerController.WasInputKeyJustPressed` (`GameplayStatics.GetPlayerController` 0) "S")
        (set `self.Curr_Dir` 1)
        (set `self.Can_move` false)
        (elif (`PlayerController.WasInputKeyJustPressed` (`GameplayStatics.GetPlayerController` 0) "A")
          (set `self.Curr_Dir` 2)
          (set `self.Can_move` false)
          (elif (`PlayerController.WasInputKeyJustPressed` (`GameplayStatics.GetPlayerController` 0) "D")
            (set `self.Curr_Dir` 3)
            (set `self.Can_move` false)))))))

(fn `Move`
  (if (== (`self.Curr_Dir`) (`self.Left`))
    (`self.K2_AddActorWorldOffset` (* (0.0 -1.0 0.0) (* 1.0 (`self.Speed`))) true)
    (set `self.Can_move` true :!label _label)
    (elif (== (`self.Curr_Dir`) (`self.Right`))
      (`self.K2_AddActorWorldOffset` (* (0.0 1.0 0.0) (* 1.0 (`self.Speed`))) true)
      (goto _label)
      (elif (== (`self.Curr_Dir`) (`self.Up`))
        (`self.K2_AddActorWorldOffset` (* (1.0 0.0 0.0) (* 1.0 (`self.Speed`))) true)
        (goto _label)
        (elif (== (`self.Curr_Dir`) (`self.Down`))
          (`self.K2_AddActorWorldOffset` (* (-1.0 0.0 0.0) (* 1.0 (`self.Speed`))) true)
          (goto _label))))))

(fn `Turn`
  (bind _returnvalue (`self.K2_GetActorLocation`))
  (bind (_worldlocation _worlddirection) (`PlayerController.DeprojectMousePositionToWorld` (`GameplayStatics.GetPlayerController` 0)))
  (`self.K2_SetActorRotation` (`KismetMathLibrary.FindLookAtRotation` _returnvalue (`KismetMathLibrary.MakeVector` (.x (+ _worldlocation (* _worlddirection (`KismetMathLibrary.VSize` (- (`SceneComponent.K2_GetComponentLocation` (`self.ShipMesh`)) (`SceneComponent.K2_GetComponentLocation` (`self.Camera`))))))) (.y (+ _worldlocation (* _worlddirection (`KismetMathLibrary.VSize` (- (`SceneComponent.K2_GetComponentLocation` (`self.ShipMesh`)) (`SceneComponent.K2_GetComponentLocation` (`self.Camera`))))))) (.z _returnvalue)))))

(fn `Turn 2`
  ;[1 1 1] if curr == prev do not turn
  (if (== (`self.Prev_Dir`) (`self.Curr_Dir`))
    _
    (elif (== (`self.Curr_Dir`) (`self.Right`))
      (`self.K2_SetActorRotation` (struct :`Yaw` 90.0))
      (elif (== (`self.Curr_Dir`) (`self.Down`))
        (`self.K2_SetActorRotation` (struct :`Yaw` 180.0))
        (elif (== (`self.Curr_Dir`) (`self.Up`))
          (`self.K2_SetActorRotation` (struct))
          (elif (== (`self.Curr_Dir`) (`self.Left`))
            (`self.K2_SetActorRotation` (struct :`Yaw` 270.0))))))))

(fn `Update`
  ;[1 1 1] Check if alive
  (if (not (`self.Dead`))
    (`self.ChickController`) ; set move
    ;[1 1 1] Check if can move
    (if (not (`self.Can_move`))
      ;[1 1 1] Move and turn towards direction
      (`self.Turn 2`)
      (`self.Move`))))

(fn `UserConstructionScript`)