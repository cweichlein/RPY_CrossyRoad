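; StripSpawner builds the initial run of strips by spawning BP_TunnelSpawner actors at BeginPlay.
; Each strip gets a random vehicle direction, spawn delay and ground type, plus a back-reference to the spawner.
; The newest strip's NextStripLocation sets where the next one spawns, chaining them in sequence.
; All strips are stored in the Strips array, and SpawnStipAtPoint appends one at the saved location.
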(event `self.ReceiveBeginPlay`
  (`self.SpawnInitialStrips`))

(event `self.ReceiveTick`
  (params (DeltaSeconds :type "Float (single-precision)")))

(fn `SetRandomValues`
  (returns (VehicleDelay :type "Float (double-precision)") (VehicleDirection :type Boolean) (GroundType :type Integer))
  (return (`KismetMathLibrary.RandomFloatInRange` 1.0 4.0) (`KismetMathLibrary.RandomBool`) (`KismetMathLibrary.RandomIntegerInRange` 0 1)))

(fn `SpawnInitialStrips`
  (for _ (range 10)
    (`/Engine/EditorBlueprintResources/StandardMacros.IsValid` (`self.NewestStrip`)
      (:`Is Valid`
        (`self.SpawnStipAtPoint`))
      (:`Is Not Valid`
        (`self.SpawnStrip` (-100.0 0.0 0.0))))))

(fn `SpawnStipAtPoint`
  (`self.SpawnStrip` (`self.NextStripLocation`)))

(fn `SpawnStrip`
  (params (SpawnLocation :type "Vector Structure"))
  (bind (_vehicledelay _vehicledirection _groundtype) (`self.SetRandomValues`))
  (bind _returnvalue (`|SpawnActorFromClass` "/Game/InfiniteMatrix/Blueprints/BP_TunnelSpawner.BP_TunnelSpawner_C" (`KismetMathLibrary.MakeTransform` (0.0 0.0 0.0)) "Undefined" "OverrideRootScale" null _vehicledirection SpawnLocation _vehicledelay (`self.StripSpacing`) _groundtype null))
  (bind _output_get (set `self.NewestStrip` _returnvalue))
  (set `/Game/InfiniteMatrix/Blueprints/BP_TunnelSpawner.StripSpawner` self _output_get)
  (set `self.NextStripLocation` (`/Game/InfiniteMatrix/Blueprints/BP_TunnelSpawner.NextStripLocation` _output_get))
  (`KismetArrayLibrary.Array_Add` (`self.Strips`) _output_get))

(fn `UserConstructionScript`)