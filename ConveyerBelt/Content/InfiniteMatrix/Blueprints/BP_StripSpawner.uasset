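; BP_StripSpawner is an actor that builds a chain of randomized BP_Strip segments starting from the player's location.
; On BeginPlay it spawns ten strips, placing the first at the player pawn and each later one at the SpawnPoint of the newest strip.
; Each new strip becomes NewestStrip, receives a reference back to the spawner and randomizes itself.
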(event `self.ReceiveBeginPlay`
  (`self.SpawnInitialStrips`))

(fn `SpawnInitialStrips`
  (for _ (range 10)
    (`/Engine/EditorBlueprintResources/StandardMacros.IsValid` (`self.NewestStrip`)
      (:`Is Valid`
        (`self.SpawnStripAtSpawnPoint`))
      (:`Is Not Valid`
        (`self.SpawnStrip` (`self.K2_GetActorLocation` (`GameplayStatics.GetPlayerPawn` 0)))))))

(fn `SpawnStrip`
  (params (SpawnLocation :type "Vector Structure"))
  (bind _returnvalue (`|SpawnActorFromClass` "/Game/InfiniteMatrix/Blueprints/BP_Strip.BP_Strip_C" (`KismetMathLibrary.MakeTransform` SpawnLocation) "Undefined" "OverrideRootScale" null null))
  (bind _output_get (set `self.NewestStrip` _returnvalue))
  (set `/Game/InfiniteMatrix/Blueprints/BP_Strip.StripSpawner` self _output_get)
  (`/Game/InfiniteMatrix/Blueprints/BP_Strip.RandomizeStrip` _output_get))

(fn `SpawnStripAtSpawnPoint`
  (`self.SpawnStrip` (`SceneComponent.K2_GetComponentLocation` (`/Game/InfiniteMatrix/Blueprints/BP_Strip.SpawnPoint` (`self.NewestStrip`)))))

(fn `UserConstructionScript`)